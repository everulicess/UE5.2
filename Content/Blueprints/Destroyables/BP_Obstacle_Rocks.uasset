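; BP_Obstacle_Rocks is a destroyable rock obstacle with health, a configurable mesh and a durability bar widget.
; When the third-person character enters its Box trigger, it shows the bar and an outline overlay material, clearing both on exit, the bar after a delay.
; Damage lowers health and updates the bar, with a short lockout between hits; at zero the actor is destroyed after a delay.
; GetDamageableType reports its damageable category.
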(event OnComponentBeginOverlap(Box)
  (params (OverlappedComponent :type Primitive%20Component%20Object%20Reference) (OtherActor :type Actor%20Object%20Reference) (OtherComp :type Primitive%20Component%20Object%20Reference) (OtherBodyIndex :type Integer) (bFromSweep :type Boolean) (SweepResult :type Hit%20Result%20Structure%20%28by%20ref%29))
  (Utilities|Casting|CastToBP_ThirdPersonCharacter OtherActor)
  (Rendering|Material|SetOverlayMaterial (Variables|Default|GetStaticMesh) (Variables|Default|GetOutline%20Material) :!class /Script/Engine.MeshComponent)
  (CallFunction|SetWidgetsVisibility "Visible"))

(event OnComponentEndOverlap(Box)
  (params (OverlappedComponent :type Primitive%20Component%20Object%20Reference) (OtherActor :type Actor%20Object%20Reference) (OtherComp :type Primitive%20Component%20Object%20Reference) (OtherBodyIndex :type Integer))
  (Utilities|Casting|CastToBP_ThirdPersonCharacter OtherActor)
  (Rendering|Material|SetOverlayMaterial (Variables|Default|GetStaticMesh) 0 :!class /Script/Engine.MeshComponent)
  (Utilities|FlowControl|Delay 1.0)
  (CallFunction|SetWidgetsVisibility "Hidden"))

(event Custom|Set%20Widgets%20Visibility
  (params (Visibility%20State :type ESlateVisibility%20Enum :default "Visible"))
  ;[1 1 1] Widgets Visibility
  (Widget|SetVisibility (Variables|Default|GetBar%20Widget) Visibility%20State))

(event EventBeginPlay
  (CallFunction|CreateWidget))

(event Collision|EventActorBeginOverlap
  (params (OtherActor :type Actor%20Object%20Reference)))

(event EventTick
  (params (DeltaSeconds :type Float%20%28single-precision%29)))

(event EventDamage
  (params (Damage :type Float%20%28double-precision%29))
  (if (not (Variables|Default|GetisGettingHit))
    (Variables|Default|SetisGettingHit true)
    (Variables|Default|SetCurrent%20Health (- (Variables|Default|GetCurrent%20Health) Damage))
    (CallFunction|UpdateWidget)))

(event EventCheckDurability
  (if (> (Variables|Default|GetCurrent%20Health) 0.0)
    (Utilities|FlowControl|Delay 0.25)
    (Variables|Default|SetisGettingHit false)
    (else
      (CallFunction|DestroyObject))))

(event EventCreateWidget
  (bind _returnvalue (UserInterface|CreateWidget "/Game/Blueprints/Widgets/Health/WBP_Destroyable_Bar.WBP_Destroyable_Bar_C"))
  (bind _output_get (Variables|Default|SetBar%20Widget _returnvalue))
  (UserInterface|Viewport|AddtoViewport _output_get 0)
  (CallFunction|SetWidgetsVisibility "Hidden")
  ;[1 1 1] Widgets Visibility
  (CallFunction|UpdateWidget))

(event EventUpdateWidget
  (Default|UpdateBar (Variables|Default|GetBar%20Widget) (/ (Variables|Default|GetCurrent%20Health) (Variables|Default|GetMax%20Health)))
  (CallFunction|CheckDurability))

(event EventDestroyObject
  (CallFunction|SetWidgetsVisibility "Hidden")
  (Utilities|FlowControl|Delay 0.5)
  (Actor|DestroyActor))

(fn ConstructionScript
  (Variables|Default|SetCurrent%20Health (Variables|Default|GetMax%20Health))
  (Components|StaticMesh|SetStaticMesh (Variables|Default|GetStaticMesh) (Variables|Default|GetDestroyableMesh)))

(fn GetDamageableType
  (return "NewEnumerator2"))