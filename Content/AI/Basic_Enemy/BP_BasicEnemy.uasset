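; BP_BasicEnemy is a melee enemy with a camera-facing health bar that appears when pawn sensing spots the third-person character.
; Attack plays a montage, and HitDetection sphere-traces between weapon sockets, damaging BPI_Damageable actors of a different damageable type.
; Incoming damage updates the bar and checks durability, with a hit flag blocking repeat hits briefly until the enemy is destroyed at depleted health.
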(event OnSeePawn(PawnSensing)
  (params (Pawn :type Pawn%20Object%20Reference))
  ;[1 1 1] Pawn Sensing
  (Utilities|Casting|CastToBP_ThirdPersonCharacter Pawn)
  (CallFunction|SetWidgetsVisibility "Visible"))

(event Custom|Set%20Widgets%20Visibility
  (params (Visibility%20State :type ESlateVisibility%20Enum :default "Visible"))
  ;[1 1 1] Widgets Visibility
  (Widget|SetVisibility (Variables|Health|GetHealth%20widget%20ref) Visibility%20State))

(event Custom|Attack
  (if (not (Variables|Combat|GetAttacking?))
    (Variables|Combat|SetAttacking? true)
    (Animation|Montage|PlayMontage (Variables|Character|GetMesh) (Utilities|Select :Index (Variables|Combat|GetAttack%20Count) :Option%200 "/Game/Animations/EnemyAnimations/Anim_Enemy_Attack_8_Montage.Anim_Enemy_Attack_8_Montage" :Option%201 "/Game/Animations/EnemyAnimations/Anim_Enemy_Attack_8_Montage.Anim_Enemy_Attack_8_Montage")
      (:then
        (Math|Integer|IncrementInt (Variables|Combat|GetAttack%20Count)))
      (:OnCompleted
        (Variables|Combat|SetAttack%20Count 0)
        (Variables|Combat|SetAttacking? false :!label _label))
      (:OnInterrupted
        (Utilities|FlowControl|Delay 3.0)
        (goto _label)))))

(event EventBeginPlay
  (CallFunction|CreateWidget)
  (CallFunction|UpdateWidget))

(event EventHitDetection
  (CallFunction|HitDetect))

(event EventTick
  (params (DeltaSeconds :type Float%20%28single-precision%29))
  (CallFunction|SetWidgetWorldRotation))

(event EventCreateWidget
  ;[1 1 1] Widget Creation
  ;;[1 1 1] Setting widget reference
  (bind _aswbp_enemy_health (Utilities|Casting|CastToWBP_Enemy_Health (UserInterface|GetWidget (Variables|Default|GetHealth%20Widget))))
  (Variables|Health|SetHealth%20widget%20ref _aswbp_enemy_health)
  (CallFunction|SetWidgetsVisibility "Hidden"))

(event EventDamage
  (params (Damage :type Float%20%28double-precision%29))
  ;[1 1 1] Receive Damage
  (if (not (Variables|Combat|GetisGettingHit))
    (Variables|Combat|SetisGettingHit true)
    (Variables|Health|SetCurrent%20Health (- (Variables|Health|GetCurrent%20Health) Damage))
    (CallFunction|UpdateWidget)))

(event EventCheckDurability
  ;[1 1 1] Durability
  (if (>= (Variables|Health|GetCurrent%20Health) 0.1)
    (Utilities|FlowControl|Delay 0.25)
    (Variables|Combat|SetisGettingHit false)
    (else
      (CallFunction|DestroyObject))))

(event EventDestroyObject
  ;[1 1 1] Destroy Object
  (Utilities|FlowControl|Delay 0.5)
  (Actor|DestroyActor))

(event EventUpdateWidget
  ;[1 1 1] Widget Update
  (Default|UpdateHealthBar (Variables|Health|GetHealth%20widget%20ref) (/ (Variables|Health|GetCurrent%20Health) (Variables|Health|GetMax%20Health)))
  (CallFunction|CheckDurability))

(fn ConstructionScript
  (Variables|Health|SetCurrent%20Health (Variables|Health|GetMax%20Health)))

(fn SetWidgetWorldRotation
  (bind _health_widget (Variables|Default|GetHealth%20Widget))
  (Transformation|SetWorldRotation _health_widget (Math|Rotator|FindLookatRotation (Transformation|GetWorldLocation _health_widget) (Transformation|GetWorldLocation (Variables|/Script/Engine.PlayerCameraManager|GetTransformComponent (Game|GetPlayerCameraManager 0)))) false false))

(fn HitDetect
  (bind _weapon_static_mesh (Variables|Default|GetWeapon%20Static%20Mesh))
  (bind _outhit (Collision|SphereTraceForObjects (Transformation|GetSocketLocation _weapon_static_mesh "Start") (Transformation|GetSocketLocation _weapon_static_mesh "End") 5e+01 (Utilities|Array|MakeArray "ObjectTypeQuery3" "ObjectTypeQuery2" "ObjectTypeQuery1") false 0 "ForOneFrame"))
  (bind _asbpi_damageable (Utilities|Casting|CastToBPI_Damageable (.HitActor (Collision|BreakHitResult _outhit))))
  (bind _type (Default|GetDamageableType _asbpi_damageable))
  (if (Utilities|Enum|NotEqual(Enum) _type (Variables|Combat|GetDamageable%20Type))
    (Default|ReceiveDamage _asbpi_damageable (Variables|Combat|GetDamage))))

(fn GetDamageableType
  (return (Variables|Combat|GetDamageable%20Type)))