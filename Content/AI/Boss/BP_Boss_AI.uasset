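; BP_Boss_AI is a boss actor that tracks health and displays it on both a screen and a world-space health bar.
; Both bars start hidden and appear when PawnSensing sees the third-person player character.
; Damage updates both bars, with a brief hit lockout between hits, then removes the screen bar and destroys the actor when health runs out.
; A function to turn the world bar toward the camera exists but is not called here.
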(event OnSeePawn(PawnSensing)
  (params (Pawn :type Pawn%20Object%20Reference))
  ;[1 1 1] Pawn Sensing
  (Utilities|Casting|CastToBP_ThirdPersonCharacter Pawn)
  (CallFunction|SetWidgetsVisibility "Visible"))

(event Custom|Set%20Widgets%20Visibility
  (params (Visibility%20State :type ESlateVisibility%20Enum :default "Visible"))
  ;[1 1 1] Widgets Visibility
  (Widget|SetVisibility (UserInterface|GetWidget (Variables|Default|GetHealth%20Widget)) Visibility%20State)
  (Widget|SetVisibility (Variables|Health|GetScreen%20Health%20Widget) Visibility%20State))

(event EventBeginPlay
  (CallFunction|CreateWidget))

(event EventTick
  (params (DeltaSeconds :type Float%20%28single-precision%29)))

(event EventDestroyObject
  ;[1 1 1] Destroy Object
  (Widget|RemovefromParent (Variables|Health|GetScreen%20Health%20Widget))
  (Utilities|FlowControl|Delay 0.5)
  (Actor|DestroyActor))

(event EventUpdateWidget
  (bind _max_health (Variables|Health|GetMax%20Health))
  (bind _current_health (Variables|Health|GetCurrent%20Health))
  (bind _returnvalue (/ _current_health _max_health))
  ;[1 1 1] Updating Widgets
  (Default|UpdateHealthPercentage (Variables|Health|GetScreen%20Health%20Widget) _returnvalue)
  (Default|UpdateHealthPercentage (Variables|Health|GetWorld%20Health%20Widget) _returnvalue))

(event EventCreateWidget
  ;[1 1 1] Creating HealthBars
  (bind _returnvalue (UserInterface|CreateWidget "/Game/Blueprints/Widgets/Health/WBP_Boss_HealthBar.WBP_Boss_HealthBar_C" (Game|GetPlayerController 0)))
  (bind _output_get (Variables|Health|SetScreen%20Health%20Widget _returnvalue))
  (UserInterface|Viewport|AddtoViewport _output_get 0)
  ;;[1 1 1] Setting world HP variable
  (bind _aswbp_boss_health_bar (Utilities|Casting|CastToWBP_Boss_HealthBar (UserInterface|GetWidget (Variables|Default|GetHealth%20Widget))))
  (Variables|Health|SetWorld%20Health%20Widget _aswbp_boss_health_bar)
  (CallFunction|SetWidgetsVisibility "Hidden"))

(event EventCheckDurability
  ;[1 1 1] Checks if it can get more damage
  (if (>= (Variables|Health|GetCurrent%20Health) 0.1)
    (Utilities|FlowControl|Delay 0.25)
    (Variables|Default|SetIsGettingHit false)
    (else
      (CallFunction|DestroyObject))))

(event EventDamage
  (params (Damage :type Float%20%28double-precision%29))
  ;[1 1 1] Damage
  (if (not (Variables|Default|GetIsGettingHit))
    (Variables|Default|SetIsGettingHit true)
    (Variables|Health|SetCurrent%20Health (- (Variables|Health|GetCurrent%20Health) Damage))
    (CallFunction|UpdateWidget)
    (CallFunction|CheckDurability)))

(fn ConstructionScript
  (Variables|Health|SetCurrent%20Health (Variables|Health|GetMax%20Health)))

(fn SetWidgetWorldRotaion
  (bind _health_widget (Variables|Default|GetHealth%20Widget))
  (Transformation|SetWorldRotation _health_widget (Math|Rotator|FindLookatRotation (Transformation|GetWorldLocation _health_widget) (Transformation|GetWorldLocation (Variables|/Script/Engine.PlayerCameraManager|GetTransformComponent (Game|GetPlayerCameraManager 0)))) false false))